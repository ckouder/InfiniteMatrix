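; BP_Enemy is a moving hazard that damages BP_Player on overlap by subtracting HealthDelta from its health.
; Each tick it drifts along world Y and Z and tumbles, with SpeedY and SpeedZ driving both movement and rotation.
; When its Sphere component overlaps BP_Tunnel, both speeds are reassigned, apparently intended to vary by a random amount.
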(event OnComponentBeginOverlap(Sphere)
  (params (OverlappedComponent :type Primitive%20Component%20Object%20Reference) (OtherActor :type Actor%20Object%20Reference) (OtherComp :type Primitive%20Component%20Object%20Reference) (OtherBodyIndex :type Integer) (bFromSweep :type Boolean) (SweepResult :type Hit%20Result%20Structure%20%28by%20ref%29))
  (Utilities|Casting|CastToBP_Tunnel OtherActor)
  (Variables|Default|SetSpeedY (stale _result))
  (Variables|Default|SetSpeedZ (stale _result)))

(event Collision|EventActorBeginOverlap
  (params (OtherActor :type Actor%20Object%20Reference))
  (bind _asbp_player (Utilities|Casting|CastToBP_Player OtherActor))
  (Default|SetHealth _asbp_player (- (Variables|/Game/InfiniteMatrix/Blueprints/BP_Player.BP_Player_C|GetHealth _asbp_player) (Variables|Default|GetHealthDelta))))

(event EventTick
  (params (DeltaSeconds :type Float%20%28single-precision%29))
  (bind _speedy (Variables|Default|GetSpeedY))
  (bind _speedz (Variables|Default|GetSpeedZ))
  (bind _returnvalue (* DeltaSeconds _speedy))
  (bind _returnvalue_2 (* DeltaSeconds _speedz))
  (Transformation|AddActorWorldOffset (Math|Vector|MakeVector 0.0 _returnvalue _returnvalue_2))
  (Class|Actor|AddActorWorldRotation (Math|Rotator|MakeRotator _returnvalue _returnvalue _returnvalue_2)))

(fn ConstructionScript)